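; Start-game character Blueprint for the KeQing model, handling eye blinking and look-at control.
; Each Tick runs FreshEye, where a timeline drives the "まばたき" (blink) morph target on the mesh.
; CloseEye sets a flag that holds the morph fully on instead and zeroes the look-at alpha.
; Two setter functions pass look-at location and alpha to the StartGameAnimInst animation instance.
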(event `self.ReceiveTick`
  (params (DeltaSeconds :type "Float (single-precision)"))
  (if (`self.IfAlwaysCloseEye`)
    (`SkeletalMeshComponent.SetMorphTarget` (`self.Mesh`) "まばたき" 1.0 true)
    (elif (`self.ReplyEyeClose`)
      (bind (_direction _eyecolseparam) (`Timeline|Timeline_0` :`NewTime` DeltaSeconds :!label _label)
        (:`Update`
          (`SkeletalMeshComponent.SetMorphTarget` (`self.Mesh`) "まばたき" _eyecolseparam true)
          (set `self.ReplyEyeClose` true))
        (:`Finished`
          (set `self.ReplyEyeClose` false)))
      (else
        (goto _label :!via `PlayFromStart`)))))

(event `CloseEye`
  (set `self.IfAlwaysCloseEye` true)
  (`self.SetLookAtTargetAlpha` 0.0))

(fn `Set Look at Target Loc`
  (params (InLoc :type "Vector Structure"))
  (bind _asstart_game_anim_inst (cast `/Game/Res/Models/KeQing/StartGameAnimInst` (`SkeletalMeshComponent.GetAnimInstance` (`self.Mesh`))))
  (set `/Game/Res/Models/KeQing/StartGameAnimInst.Look At Location` InLoc _asstart_game_anim_inst))

(fn `SetLookAtTargetAlpha`
  (params (InParams :type "Float (double-precision)"))
  (bind _asstart_game_anim_inst (cast `/Game/Res/Models/KeQing/StartGameAnimInst` (`SkeletalMeshComponent.GetAnimInstance` (`self.Mesh`))))
  (set `/Game/Res/Models/KeQing/StartGameAnimInst.LookAtAlpha` InParams _asstart_game_anim_inst))

(fn `UserConstructionScript`)