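; BP_GlobalMaterialSettings is an actor that publishes the scene's directional light to the MPC_GlobalParams material parameter collection.
; It finds a DirectionalLight actor on BeginPlay, or during construction if none is set.
; SetMaterialParams writes the light's forward vector, color and intensity into the collection.
; It runs in the construction script for editor updates and every Tick at runtime.
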(event `self.ReceiveBeginPlay`
  (bind _returnvalue (`GameplayStatics.GetActorOfClass` "/Script/Engine.DirectionalLight"))
  (set `self.DirectionalLight` _returnvalue))

(event `self.ReceiveTick`
  (params (DeltaSeconds :type "Float (single-precision)"))
  (`self.SetMaterialParams` (`self.DirectionalLight`)))

(fn `SetMaterialParams`
  (params (DirLight :type "Light Object Reference"))
  (bind _lightcomponent (`Light.LightComponent` DirLight))
  (set `self.LightDirectionMatVector` (`KismetMathLibrary.Conv_VectorToLinearColor` (`KismetMathLibrary.GetForwardVector` (`self.K2_GetActorRotation` DirLight))))
  (`KismetMaterialLibrary.SetVectorParameterValue` "/Game/Res/Materials/MPC_GlobalParams.MPC_GlobalParams" "LightDirection" (`self.LightDirectionMatVector`))
  (`KismetMaterialLibrary.SetVectorParameterValue` "/Game/Res/Materials/MPC_GlobalParams.MPC_GlobalParams" "LightColor" (`LightComponentBase.GetLightColor` _lightcomponent))
  (`KismetMaterialLibrary.SetScalarParameterValue` "/Game/Res/Materials/MPC_GlobalParams.MPC_GlobalParams" "LightIntensity" (`LightComponentBase.Intensity` _lightcomponent)))

(fn `UserConstructionScript`
  (`/Engine/EditorBlueprintResources/StandardMacros.IsValid` (`self.DirectionalLight`)
    (:`Is Valid`
      _)
    (:`Is Not Valid`
      (bind _returnvalue (`GameplayStatics.GetActorOfClass` "/Script/Engine.DirectionalLight"))
      (bind _output_get (set `self.DirectionalLight` _returnvalue))))
  (`self.SetMaterialParams` _output_get))