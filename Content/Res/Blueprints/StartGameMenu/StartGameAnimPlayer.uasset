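; StartGameAnimPlayer is a start-menu actor that drives the intro camera and character presentation.
; Each tick it traces under the mouse cursor and, when an actor is hit, points the target character's look-at at the hit location.
; Its Play function blends the player view to a target camera with ease-in-out and plays the first LevelSequenceActor found in the level.
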(event `self.ReceiveTick`
  (params (DeltaSeconds :type "Float (single-precision)"))
  (bind (_bblockinghit _binitialoverlap _time _distance _location _impactpoint _normal _impactnormal _physmat _hitactor) (`GameplayStatics.BreakHitResult` (`PlayerController.GetHitResultUnderCursorForObjects` (`GameplayStatics.GetPlayerController` 0) (`self.Object Types`) true)))
  (`/Engine/EditorBlueprintResources/StandardMacros.IsValid` _hitactor
    (:`Is Valid`
      (`/Game/Res/Models/KeQing/BP_StartGameCharacter.Set Look at Target Loc` (`self.TargetCharacter`) _location))))

(fn `Play`
  (`PlayerController.SetViewTargetWithBlend` (`GameplayStatics.GetPlayerController` 0) (`self.TargetCamera`) 1.0 "VTBlend_EaseInOut" 3.0 false)
  (bind _returnvalue (`GameplayStatics.GetActorOfClass` "/Script/LevelSequence.LevelSequenceActor"))
  (`/Engine/EditorBlueprintResources/StandardMacros.IsValid` _returnvalue
    (:`Is Valid`
      (`MovieSceneSequencePlayer.Play` (`LevelSequenceActor.SequencePlayer` _returnvalue)))))

(fn `UserConstructionScript`)