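; Character showcase actor that displays a skeletal mesh on a spring-arm camera, with mouse-wheel zoom and left-drag rotation.
; Tick smooths arm length, yaws the mesh and pitches the clamped arm from eased mouse input, or lerps both back after a reset.
; ChangeCharacter swaps the mesh, resets the view, sets arm height from the Head socket and picks a color by entity ID.
; That color blends into SkyAtmosphere scattering and height fog as the backdrop.
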(event `self.ReceiveBeginPlay`
  (bind _returnvalue (`GameplayStatics.GetActorOfClass` "/Script/Engine.SkyAtmosphere"))
  (set `self.SkyAtomsphere` _returnvalue)
  (bind _returnvalue_2 (`GameplayStatics.GetActorOfClass` "/Script/Engine.ExponentialHeightFog"))
  (set `self.Fog` _returnvalue_2))

(event `InputAxisKey|MouseWheelAxis`
  (params (AxisValue :type "Float (single-precision)"))
  ;[1 1 1] 相机距离缩放功能
  (if (not (== AxisValue 0.0))
    (set `self.TargetArmLength` (`KismetMathLibrary.FClamp` (- (`SpringArmComponent.TargetArmLength` (`self.SpringArm`)) (* AxisValue 20.0)) (`self.MinCameraDistance`) (`self.MaxCameraDistance`)))))

(event `Key|LeftMouseButton`
  (params (Key :type "Key Structure"))
  (:`Pressed`
    (set `self.EnableRotateCharacter` true))
  (:`Released`
    (set `self.EnableRotateCharacter` false)))

(event `InputVectorAxis|Mouse2D`
  (params (AxisValue :type "Vector Structure"))
  (bind _mousexy (`self.MouseXY`))
  (if (`self.EnableRotateCharacter`)
    (set `self.MouseXY` (`KismetMathLibrary.VLerp` _mousexy AxisValue 0.2))
    (else
      (set `self.MouseXY` (`KismetMathLibrary.VLerp` _mousexy (0.0 0.0 0.0) 0.05)))))

(event `self.ReceiveTick`
  (params (DeltaSeconds :type "Float (single-precision)"))
  (bind _springarm (`self.SpringArm`))
  (bind _returnvalue (* DeltaSeconds (`self.CharacterRotatorSpeed`)))
  (bind (_relativerotation_roll _relativerotation_pitch _relativerotation_yaw) (`KismetMathLibrary.BreakRotator` (`SceneComponent.RelativeRotation` _springarm)))
  (bind _returnvalue_2 (`KismetMathLibrary.RLerp` (`SceneComponent.RelativeRotation` (`self.SpringArm`)) (struct :`Yaw` 180.0) 0.2 true))
  (bind _returnvalue_3 (`KismetMathLibrary.RLerp` (`SceneComponent.RelativeRotation` (`self.SkeletalMesh`)) (struct :`Yaw` -90.0) 0.2))
  (set `SpringArmComponent.TargetArmLength` (`KismetMathLibrary.Lerp` (`SpringArmComponent.TargetArmLength` (`self.SpringArm`)) (`self.TargetArmLength`) (* DeltaSeconds (`self.CameraDistanceChangeSpeed`))) (`self.SpringArm`))
  (`self.ChangeBGColorSmooth`)
  (if (`self.bRset`)
    (`SceneComponent.K2_SetRelativeRotation` (`self.SpringArm`) _returnvalue_2 false false)
    (`SceneComponent.K2_SetRelativeRotation` (`self.SkeletalMesh`) _returnvalue_3 false false)
    (if (and (== _returnvalue_2 (struct :`Yaw` 180.0) :`ErrorTolerance` 0.1) (== _returnvalue_3 (struct :`Yaw` -90.0) :`ErrorTolerance` 0.1))
      (set `self.bRset` false))
    (else
      (`SceneComponent.K2_AddLocalRotation` (`self.SkeletalMesh`) (`KismetMathLibrary.MakeRotator` 0.0 0.0 (* _returnvalue (.x (`self.MouseXY`)) -1.0)) false false)
      (`SceneComponent.K2_AddLocalRotation` _springarm (`KismetMathLibrary.MakeRotator` 0.0 (* _returnvalue (.y (`self.MouseXY`)))) false false)
      (`SceneComponent.K2_SetRelativeRotation` (`self.SpringArm`) (`KismetMathLibrary.MakeRotator` _relativerotation_roll (`KismetMathLibrary.ClampAngle` _relativerotation_pitch -45.0 45.0) _relativerotation_yaw) false false))))

(fn `ChangeBGColorSmooth`
  (bind _skyatmospherecomponent (`SkyAtmosphere.SkyAtmosphereComponent` (`self.SkyAtomsphere`)))
  (bind _returnvalue (`KismetMathLibrary.LinearColorLerp` (`SkyAtmosphereComponent.RayleighScattering` _skyatmospherecomponent) (`self.TargetBGColor`) 0.1))
  (`SkyAtmosphereComponent.SetRayleighScattering` _skyatmospherecomponent _returnvalue)
  (`ExponentialHeightFogComponent.SetFogInscatteringColor` (`ExponentialHeightFog.Component` (`self.Fog`)) (* _returnvalue (struct :`R` 0.572917 :`G` 0.572917 :`B` 0.572917 :`A` 1.0))))

(fn `ChangeCharacter`
  (params (InItem :type "CharacterEntryItem Object Reference"))
  (bind (_entityparams_entityid _entityparams_displayname _entityparams_skeletalmesh) (break `EntityParams` (`CharacterEntryItem.EntityParams` InItem)))
  (bind _skeletalmesh (`self.SkeletalMesh`))
  (bind (_returnvalue_x _returnvalue_y _returnvalue_z) (`KismetMathLibrary.BreakVector` (- (`SceneComponent.GetSocketLocation` _skeletalmesh "Head") (`SceneComponent.K2_GetComponentLocation` _skeletalmesh))))
  (`SkinnedMeshComponent.SetSkinnedAssetAndUpdate` (`self.SkeletalMesh`) (`|ConvertAsset` _entityparams_skeletalmesh) true)
  (`self.Reset`)
  (`|ExecutionSequence`
    (:`then_0`
      (if (== _entityparams_entityid 1001)
        (set `self.TargetBGColor` (struct :`R` 0.402759 :`G` 1.0 :`B` 0.361772 :`A` 1.0))
        (else
          (set `self.TargetBGColor` (struct :`R` 0.758552 :`G` 0.155993 :`B` 1.0 :`A` 1.0)))))
    (:`then_1`
      (`SceneComponent.K2_SetRelativeLocation` (`self.SpringArm`) (`KismetMathLibrary.MakeVector` 0.0 0.0 _returnvalue_z) false false))))

(fn `Reset`
  (set `self.TargetArmLength` 200.0)
  (set `self.bRset` true))

(fn `UserConstructionScript`)