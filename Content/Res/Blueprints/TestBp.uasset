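; TestBp is a test actor that spawns a turret and an enemy, then drives the enemy toward the turret's spawn point.
; BeginPlay constructs an EntityCreator, creates the turret at the actor's transform and, after a short delay, creates the enemy offset along world +Y.
; Tick feeds forced movement input along world -Y to the stored enemy while it is valid.
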(event `self.ReceiveBeginPlay`
  (bind (_returnvalue_location _returnvalue_rotation _returnvalue_scale) (`KismetMathLibrary.BreakTransform` (`self.GetTransform`)))
  (bind _returnvalue (`|GenericCreateObject` "/Script/TowerDefence.EntityCreator" self))
  (bind _output_get (set `self.EntityCreator` _returnvalue))
  (`EntityCreator.CreateTurrent` _output_get 1001 (`self.GetTransform`))
  (`KismetSystemLibrary.Delay` 0.2)
  (bind _returnvalue_2 (`EntityCreator.CreateEnemy` _output_get 1001 (`KismetMathLibrary.MakeTransform` (+ _returnvalue_location (0.0 300.0 0.0)) _returnvalue_rotation _returnvalue_scale)))
  (set `self.NewVar_1` _returnvalue_2))

(event `self.ReceiveTick`
  (params (DeltaSeconds :type "Float (single-precision)"))
  (bind _newvar_1 (`self.NewVar_1`))
  (`/Engine/EditorBlueprintResources/StandardMacros.IsValid` _newvar_1
    (:`Is Valid`
      (`Pawn.AddMovementInput` _newvar_1 (0.0 -1.0 0.0) 1.0 true))))

(fn `UserConstructionScript`)